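; BP_W1GM is a game mode Blueprint that fills the level with a square grid of BP_Point actors when play begins.
; SpawnPoints uses nested loops, stepping X for each row and resetting then stepping Y within it, to place evenly spaced points at ground-plane Z zero.
; Spawns adjust around collisions or fail if still blocked, and each result is appended to the AllPoints array.
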(event `self.ReceiveBeginPlay`
  (`self.Spawn Points`))

(fn `Spawn Points`
  (locals (LocX :type "Float (double-precision)" :default 3650.0) (LocY :type "Float (double-precision)"))
  (for _ (range 72)
    (set `local.LocX` (- (`local.LocX`) 100.0))
    (set `local.LocY` 3550.0)
    (for _ (range 72)
      (bind _returnvalue (`|SpawnActorFromClass` "/Game/_Game/Point/BP_Point.BP_Point_C" (`KismetMathLibrary.Conv_VectorToTransform` (`KismetMathLibrary.MakeVector` (`local.LocX`) (`local.LocY`))) "AdjustIfPossibleButDontSpawnIfColliding" "MultiplyWithRoot" null null))
      (`KismetArrayLibrary.Array_Add` (`self.AllPoints`) _returnvalue)
      (set `local.LocY` (- (`local.LocY`) 100.0)))))

(fn `UserConstructionScript`)